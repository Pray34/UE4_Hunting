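; BP_Bullet is an explosive projectile actor with a limited lifespan.
; Its first sphere overlap with a non-owner spawns an explosion and applies radial damage with falloff, hiding mesh and sphere if damage lands.
; Blocking hits on non-owners destroy it without exploding, and debug prints and a debug sphere remain active.
; RadialForce is configured but never fired, and the enemy knockback and alternative damage nodes are unwired.
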(event `self.ReceiveBeginPlay`
  (`self.SetLifeSpan` 10.0)
  (`RadialForceComponent.AddObjectTypeToAffect` (`self.RadialForce`) "ObjectTypeQuery2"))

(event `self.Sphere.OnComponentHit`
  (params (HitComponent :type "PrimitiveComponent Object Reference") (OtherActor :type "Actor Object Reference") (OtherComp :type "PrimitiveComponent Object Reference") (NormalImpulse :type "Vector Structure") (Hit :type "HitResult Structure (by ref)"))
  (if (!= OtherActor (`self.GetOwner`))
    (`KismetSystemLibrary.PrintString` "Sphere Hit")
    (`self.K2_DestroyActor`)))

(event `self.ReceiveHit`
  (params (MyComp :type "PrimitiveComponent Object Reference") (Other :type "Actor Object Reference") (OtherComp :type "PrimitiveComponent Object Reference") (bSelfMoved :type Boolean) (HitLocation :type "Vector Structure") (HitNormal :type "Vector Structure") (NormalImpulse :type "Vector Structure") (Hit :type "HitResult Structure (by ref)"))
  (if (!= Other (`self.GetOwner`))
    (`KismetSystemLibrary.PrintString` "Actor Hit")
    (`self.K2_DestroyActor`)))

(event `self.Sphere.OnComponentBeginOverlap`
  (params (OverlappedComponent :type "PrimitiveComponent Object Reference") (OtherActor :type "Actor Object Reference") (OtherComp :type "PrimitiveComponent Object Reference") (OtherBodyIndex :type Integer) (bFromSweep :type Boolean) (SweepResult :type "HitResult Structure (by ref)"))
  (bind _bulletlocation (`self.BulletLocation`))
  (if (!= OtherActor (`self.GetOwner`))
    (`/Engine/EditorBlueprintResources/StandardMacros.DoOnce` false
      (:`Completed`
        (set `self.BulletLocation` (`SceneComponent.K2_GetComponentLocation` OverlappedComponent))
        (`KismetSystemLibrary.PrintString` (`KismetSystemLibrary.GetDisplayName` OverlappedComponent) true true (struct :`G` 0.283243 :`B` 1.0 :`A` 1.0))
        (`KismetSystemLibrary.DrawDebugSphere` _bulletlocation 300.0 36 (struct :`R` 1.0 :`G` 0.305312 :`A` 1.0) 1.0 0.5)
        (`GameplayStatics.SpawnEmitterAtLocation` "/Game/FXVarietyPack/Particles/P_ky_explosion.P_ky_explosion" _bulletlocation (struct) (0.5 0.5 0.5))
        (bind _returnvalue (`GameplayStatics.ApplyRadialDamageWithFalloff` 50.0 10.0 _bulletlocation 100.0 300.0 0.5 null (`|MakeArray` self (`self.GetOwner` self) :!type "Actor Object Reference") self null))
        (if _returnvalue
          (`SceneComponent.SetVisibility` (`self.StaticMesh`) false false)
          (`SceneComponent.SetVisibility` (`self.Sphere`) false false))))))

(fn `UserConstructionScript`)