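; Enemy character Blueprint that reacts to damage with physical knockback from bullet explosions and prints debug text for each hit.
; On radial damage it zeroes the walkable floor angle, fires the BP_Bullet damage causer's RadialForce impulse, then restores the angle after a short delay.
; A failed bullet cast stops the chain before that restore.
; Other impulse experiments remain disconnected and never run.
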(event `self.ReceiveAnyDamage`
  (params (Damage :type "Float (single-precision)") (DamageType :type "DamageType Object Reference") (InstigatedBy :type "Controller Object Reference") (DamageCauser :type "Actor Object Reference"))
  (`KismetSystemLibrary.PrintString` "Any" true true (struct :`R` 1.0 :`B` 0.097209 :`A` 1.0) 3.0))

(event `self.ReceiveRadialDamage`
  (params (DamageReceived :type "Float (single-precision)") (DamageType :type "DamageType Object Reference") (Origin :type "Vector Structure") (HitInfo :type "HitResult Structure (by ref)") (InstigatedBy :type "Controller Object Reference") (DamageCauser :type "Actor Object Reference"))
  (`KismetSystemLibrary.PrintString` "Radial" true true (struct :`R` 1.0 :`B` 0.097209 :`A` 1.0) 3.0)
  (`CharacterMovementComponent.SetWalkableFloorAngle` (`self.CharacterMovement`) 0.0)
  (bind _asbp_bullet (cast `/Game/BP_SubObject/BP_Weapon/BP_Bullet` DamageCauser))
  (`RadialForceComponent.FireImpulse` (`/Game/BP_SubObject/BP_Weapon/BP_Bullet.RadialForce` _asbp_bullet))
  (`KismetSystemLibrary.Delay` 0.5)
  (`CharacterMovementComponent.SetWalkableFloorAngle` (`self.CharacterMovement`) 45.0))

(event `self.ReceiveTick`
  (params (DeltaSeconds :type "Float (single-precision)")))

(fn `UserConstructionScript`)